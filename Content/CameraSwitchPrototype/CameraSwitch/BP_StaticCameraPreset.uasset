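; BP_StaticCameraPreset is a camera preset for the CameraSwitch prototype, configured from a CameraMode variable.
; Its Construction Script calls SetDefaultParameters, which applies that data to the spring arm's transform and collision and the camera's FOV and projection.
; It also caches follow, axis-ignore, blend time and desired-rotation settings, showing DesiredForwardDirection only when that rotation is used.
; Ortho width reuses the spring arm's distance to the player.
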(fn ConstructionScript
  (CallFunction|SetDefaultParameters))

(fn SetDefaultParameters
  (bind _camera (Variables|Default|GetCamera))
  (bind _cameramode (Variables|Default|GetCameraMode))
  (bind _cameramode_2 (Variables|Default|GetCameraMode))
  (bind _springarm (Variables|Default|GetSpringArm))
  (bind _cameramode_3 (Variables|Default|GetCameraMode))
  (bind _movementandcollision (Variables|/Game/CameraSwitchPrototype/CameraSwitch/CameraDataAssets/PDA_CameraModeConfig.PDA_CameraModeConfig_C|GetMovementAndCollision _cameramode_3))
  (bind _springarmtransform (Variables|/Game/CameraSwitchPrototype/CameraSwitch/CameraDataAssets/PDA_CameraModeConfig.PDA_CameraModeConfig_C|GetSpringArmTransform _cameramode_3))
  (Utilities|FlowControl|Sequence
    (:then_0
      (bind _output_get (Variables|Controls|SetUseDesiredRotation (Variables|/Game/CameraSwitchPrototype/CameraSwitch/CameraDataAssets/PDA_CameraModeConfig.PDA_CameraModeConfig_C|GetUseDesiredForwardVector _cameramode_3)))
      (Rendering|SetVisibility (Variables|Default|GetDesiredForwardDirection) _output_get false))
    (:then_1
      (Transformation|SetRelativeRotation _springarm (.rotation _springarmtransform) false false)
      (Variables|/Script/Engine.SpringArmComponent|SetTargetArmLength _springarm (.distancetoplayer _springarmtransform))
      (Variables|/Script/Engine.SpringArmComponent|SetTargetOffset _springarm (.offsetfromplayer _springarmtransform)))
    (:then_2
      (Variables|Default|SetFollowPlayer (.followplayer _movementandcollision))
      (Variables|/Script/Engine.SpringArmComponent|SetbDoCollisionTest _springarm (.docollisiontest _movementandcollision))
      (Variables|/Script/Engine.SpringArmComponent|SetProbeChannel _springarm (.probechannel _movementandcollision))
      (Variables|Controls|SetIgnoreXAxis (.ignorexmove _movementandcollision))
      (Variables|Controls|SetIgnoreYAxis (.ignoreymove _movementandcollision)))
    (:then_3
      (Camera|SetFieldOfView _camera (Variables|/Game/CameraSwitchPrototype/CameraSwitch/CameraDataAssets/PDA_CameraModeConfig.PDA_CameraModeConfig_C|GetFOV _cameramode))
      (Variables|Default|SetBlendTime (Variables|/Game/CameraSwitchPrototype/CameraSwitch/CameraDataAssets/PDA_CameraModeConfig.PDA_CameraModeConfig_C|GetBlendTime _cameramode))
      (Class|CameraComponent|SetProjectionMode _camera (select (Variables|/Game/CameraSwitchPrototype/CameraSwitch/CameraDataAssets/PDA_CameraModeConfig.PDA_CameraModeConfig_C|GetIsOrthographic _cameramode_2) "Orthographic" "Perspective"))
      (Class|CameraComponent|SetOrthoWidth _camera (.distancetoplayer (Variables|/Game/CameraSwitchPrototype/CameraSwitch/CameraDataAssets/PDA_CameraModeConfig.PDA_CameraModeConfig_C|GetSpringArmTransform _cameramode_2))))))