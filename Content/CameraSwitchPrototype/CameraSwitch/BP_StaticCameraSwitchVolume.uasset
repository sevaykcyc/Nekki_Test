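; Trigger volume that switches the test character's camera to a referenced static camera preset and restores the default third-person view.
; Entering the Enter volume passes the preset's blend time, follow setting and chosen rotation to the character's camera manager component, or prints a warning without a preset.
; Overlapping the Exit volume resets the camera.
; An optional flag also resets on leaving the Enter volume, with the construction script hiding the Exit volume.
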(event OnComponentBeginOverlap(Volume_Enter)
  (params (OverlappedComponent :type Primitive%20Component%20Object%20Reference) (OtherActor :type Actor%20Object%20Reference) (OtherComp :type Primitive%20Component%20Object%20Reference) (OtherBodyIndex :type Integer) (bFromSweep :type Boolean) (SweepResult :type Hit%20Result%20Structure%20%28by%20ref%29))
  ;[0.3781 0.3781 0.3781] On player overlap set In Camera Mode
  (bind _asbp_test_character (Utilities|Casting|CastToBP_TestCharacter OtherActor))
  (CallFunction|SetCameraData _asbp_test_character))

(event OnComponentBeginOverlap(Volume_Exit)
  (params (OverlappedComponent :type Primitive%20Component%20Object%20Reference) (OtherActor :type Actor%20Object%20Reference) (OtherComp :type Primitive%20Component%20Object%20Reference) (OtherBodyIndex :type Integer) (bFromSweep :type Boolean) (SweepResult :type Hit%20Result%20Structure%20%28by%20ref%29))
  ;[0.3656 0.3656 0.3656] On player exit set Default ThirdPerson perspective
  (bind _asbp_test_character (Utilities|Casting|CastToBP_TestCharacter OtherActor))
  (Default|ResettoDefault (Variables|/Game/CameraSwitchPrototype/PlayerCharacter/BP_TestCharacter.BP_TestCharacter_C|GetBP_CameraManagerComponemnt _asbp_test_character)))

(event OnComponentEndOverlap(Volume_Enter)
  (params (OverlappedComponent :type Primitive%20Component%20Object%20Reference) (OtherActor :type Actor%20Object%20Reference) (OtherComp :type Primitive%20Component%20Object%20Reference) (OtherBodyIndex :type Integer))
  ;[0.3656 0.3656 0.3656] On player exit set Default ThirdPerson perspective
  (if (Variables|Default|GetResetOnEndOverlapEnter) ; for the other sides of the trigger, where the Exit volume is missing
    (bind _asbp_test_character (Utilities|Casting|CastToBP_TestCharacter OtherActor))
    (Default|ResettoDefault (Variables|/Game/CameraSwitchPrototype/PlayerCharacter/BP_TestCharacter.BP_TestCharacter_C|GetBP_CameraManagerComponemnt _asbp_test_character))))

(fn ConstructionScript
  (Rendering|SetVisibility (Variables|Default|GetVolume_Exit) (not (Variables|Default|GetResetOnEndOverlapEnter)) false) ; Hide VolumeExit, if exiting VolumeEnter resets camera
)

(fn SetCameraData
  (params (PlayerActor :type BP%20Test%20Character%20Object%20Reference))
  (bind _camerapresetref (Variables|Default|GetCameraPresetRef))
  (Utilities|IsValid (Variables|Default|GetCameraPresetRef)
    (:Is%20Valid
      (Default|SetNewView (Variables|/Game/CameraSwitchPrototype/PlayerCharacter/BP_TestCharacter.BP_TestCharacter_C|GetBP_CameraManagerComponemnt PlayerActor) _camerapresetref (Variables|/Game/CameraSwitchPrototype/CameraSwitch/BP_StaticCameraPreset.BP_StaticCameraPreset_C|GetBlendTime _camerapresetref) (Variables|/Game/CameraSwitchPrototype/CameraSwitch/BP_StaticCameraPreset.BP_StaticCameraPreset_C|GetFollowPlayer _camerapresetref) (Math|Rotator|SelectRotator (Transformation|GetWorldRotation (Variables|/Game/CameraSwitchPrototype/CameraSwitch/BP_StaticCameraPreset.BP_StaticCameraPreset_C|GetDesiredForwardDirection _camerapresetref)) (Transformation|GetWorldRotation (Variables|/Game/CameraSwitchPrototype/CameraSwitch/BP_StaticCameraPreset.BP_StaticCameraPreset_C|GetSpringArm _camerapresetref)) (Variables|/Game/CameraSwitchPrototype/CameraSwitch/BP_StaticCameraPreset.BP_StaticCameraPreset_C|GetUseDesiredRotation _camerapresetref))))
    (:Is%20Not%20Valid
      (Development|PrintString (Utilities|String|Append (Utilities|GetDisplayName self) ": CameraPresetRef = null") true true "(R=1.000000,G=0.000000,B=0.021217,A=1.000000)") ; Reminder if CameraPresetRef configured incorrectly
    )))

(fn ResetCamera
  (params (PlayerActor :type BP%20Test%20Character%20Object%20Reference))
  (Default|ResettoDefault (Variables|/Game/CameraSwitchPrototype/PlayerCharacter/BP_TestCharacter.BP_TestCharacter_C|GetBP_CameraManagerComponemnt PlayerActor)))