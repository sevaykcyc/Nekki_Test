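; Player camera-switch component that blends the view to preset camera actors and back to the player pawn.
; For follow cameras, it spawns and attaches a duplicate to preserve the preset's transform, destroying it after reset.
; It stores a flattened camera rotation as ForwardDirection for forward and right vector calculations.
; Interface messages block pawn input during transitions, with a retriggerable delay unblocking it afterward.
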(event Custom|CameraSwitchingProcess
  (params (Delay :type Float%20%28double-precision%29) (Resetting :type Boolean))
  (Utilities|FlowControl|RetriggerableDelay (+ Delay 0.1))
  (Class|BPIPlayerSwitchCamera|BlockInputWhileSwitching(Message) (Game|Player|GetPlayerPawn 0) false)
  (if Resetting
    (CallFunction|DestroyDuplicate (Variables|Default|GetCurrentCustomCamera))))

(event Custom|DestroyDuplicate
  (params (Duplicate :type BP%20Static%20Camera%20Preset%20Object%20Reference))
  (Utilities|IsValid Duplicate
    (:Is%20Valid
      (Actor|DestroyActor Duplicate)
      (Variables|Default|SetCurrentCustomCamera 0))))

(fn SetNewView
  (params (CameraActor :type BP%20Static%20Camera%20Preset%20Object%20Reference) (BlendTime :type Float%20%28double-precision%29) (FollowPlayer :type Boolean) (CamRotation :type Rotator))
  (Utilities|FlowControl|Sequence
    (:then_0
      ;[1 1 1 0.3] Set a Static Rotation for further calculation of Forward and Right Vectors
      (Variables|Default|SetForward%20Direction (CallFunction|OrientRotation CamRotation)))
    (:then_1
      ;[1 1 1 0.3] Set New Camera perspective
      (if FollowPlayer
        (bind _returnvalue (Game|SpawnActorfromClass (Utilities|GetClass CameraActor) (Transformation|GetActorTransform CameraActor) "Undefined" "MultiplyWithRoot" 0 0)) ; Spawn duplicate for maintaining basic transforms on the original preset
        (bind _output_get (Variables|Default|SetCurrentCustomCamera _returnvalue))
        (Variables|/Game/CameraSwitchPrototype/CameraSwitch/BP_StaticCameraPreset.BP_StaticCameraPreset_C|SetCameraMode _output_get (Variables|/Game/CameraSwitchPrototype/CameraSwitch/BP_StaticCameraPreset.BP_StaticCameraPreset_C|GetCameraMode CameraActor))
        (Default|SetDefaultParameters _output_get)
        (Transformation|AttachActorToActor _output_get (Game|Player|GetPlayerPawn 0) "" "SnapToTarget" "KeepRelative" "KeepRelative" true)
        (else
          (Variables|Default|SetCurrentCustomCamera CameraActor)))
      (Game|Player|SetViewTargetwithBlend (Game|GetPlayerController 0) (Variables|Default|GetCurrentCustomCamera) BlendTime "VTBlend_Linear" 1.0 true)
      ;[1 1 1 0.3] Block Input while switching
      (Class|BPIPlayerSwitchCamera|BlockInputWhileSwitching(Message) (Game|Player|GetPlayerPawn 0) true)
      (CallFunction|CameraSwitchingProcess BlendTime false))))

(fn ResettoDefault
  (bind _returnvalue (Game|Player|GetPlayerPawn 0))
  (Class|BPIPlayerSwitchCamera|ResetPlayerCamera(Message) _returnvalue)
  (Game|Player|SetViewTargetwithBlend (Game|GetPlayerController 0) _returnvalue 1.0 "VTBlend_Linear" 1.0 false)
  (Utilities|IsValid (Variables|Default|GetCurrentCustomCamera)
    (:Is%20Valid
      (if (Variables|/Game/CameraSwitchPrototype/CameraSwitch/BP_StaticCameraPreset.BP_StaticCameraPreset_C|GetFollowPlayer (Variables|Default|GetCurrentCustomCamera))
        _
        (else
          (Variables|Default|SetCurrentCustomCamera 0 :!label _label))))
    (:Is%20Not%20Valid
      (goto _label)))
  ;[1 1 1 0.3] Block Input While resetting
  (Class|BPIPlayerSwitchCamera|BlockInputWhileSwitching(Message) (Game|Player|GetPlayerPawn 0) true)
  (CallFunction|CameraSwitchingProcess 0.5 true))

(fn OrientRotation
  (params (CameraWorldRotation :type Rotator))
  (bind _returnvalue (Math|Vector|GetRightVector CameraWorldRotation))
  (bind _returnvalue_2 (Math|Vector|MakeVector (.x _returnvalue) (.y _returnvalue) 0.0))
  (return (Math|Rotator|MakeRotfromXY (Math|Vector|Normalize (Math|Vector|RotateVectorAroundAxis _returnvalue_2 -9e+01 "0.000000,0.000000,1.000000")) _returnvalue_2)))